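; Interactive switchboard puzzle where the player flips four switches to trigger StartFleeing.
; Interact blends the camera to the board, disables player input and enables mouse clicking.
; Each debounced, FlipFlop-driven click plays a sound and timeline rotation, then nudges two gauge needles via MoveComponentTo and checks completion.
; Once all four switches are on, Done fetches BP_Light actors, calls StartFleeing and restores player view and control.
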(event `/Game/Switch/BPI_Main.Interact`
  (bind _returnvalue (`GameplayStatics.GetPlayerController` 0))
  (set `self.ins` true)
  (`WidgetBlueprintLibrary.SetFocusToGameViewport`)
  (`/Engine/EditorBlueprintResources/StandardMacros.DoOnce` false :!label _label
    (:`Completed`
      (`|ExecutionSequence`
        (:`then_0`
          (`/Engine/EditorBlueprintResources/StandardMacros.FlipFlop`
            (:`A`
              (bind _asbp_fpshooter (cast `/Game/Variant_Shooter/Blueprints/FirstPerson/BP_FPShooter` (`GameplayStatics.GetPlayerCharacter` 0)))
              (`self.DisableInput` _asbp_fpshooter _returnvalue)
              (`PlayerController.SetViewTargetWithBlend` _returnvalue self 1.0 "VTBlend_Linear" 0.0 false)
              (set `PlayerController.bShowMouseCursor` true _returnvalue)
              (`SceneComponent.SetVisibility` (`self.BP_MasterItem`) false false)
              (set `PlayerController.bEnableClickEvents` true _returnvalue))))
        (:`then_1`
          (`KismetSystemLibrary.Delay` 1.1)
          (goto _label :!via `Reset`))))))

(event `Done`
  (bind _returnvalue (`GameplayStatics.GetPlayerController` 0))
  (if (and (`self.Switch01On`) (`self.Switch02On`) (`self.Switch03On`) (`self.Switch04On`))
    (set `self.SwitchesAll` true)
    (`GameplayStatics.GetAllActorsOfClass` "/Game/Variant_Shooter/Blueprints/Pickups/BP_Light.BP_Light_C")
    (`self.StartFleeing`)
    (`KismetSystemLibrary.PrintString` "Hello")
    (`PlayerController.SetViewTargetWithBlend` _returnvalue (`GameplayStatics.GetPlayerCharacter` 0) 1.0 "VTBlend_Linear" 0.0 false)
    (set `PlayerController.bShowMouseCursor` false _returnvalue)
    (set `PlayerController.bEnableClickEvents` false _returnvalue)
    (`WidgetBlueprintLibrary.SetInputMode_GameOnly` _returnvalue true)
    (bind _asbp_fpshooter (cast `/Game/Variant_Shooter/Blueprints/FirstPerson/BP_FPShooter` (`GameplayStatics.GetPlayerCharacter` 0)))
    (`self.EnableInput` _asbp_fpshooter (`GameplayStatics.GetPlayerController` 0))))

(event `self.ReceiveBeginPlay`
  (set `self.needle01 Rotation` (`SceneComponent.RelativeRotation` (`self.SM_Board_Needle`)))
  (set `self.needle02 Rotation` (`SceneComponent.RelativeRotation` (`self.SM_Board_Needle1`))))

(event `self.SM_Switch.OnClicked`
  (params (TouchedComponent :type "PrimitiveComponent Object Reference") (ButtonPressed :type "Key Structure"))
  (`KismetSystemLibrary.PrintString` "1")
  (`WidgetBlueprintLibrary.SetFocusToGameViewport`)
  (`/Engine/EditorBlueprintResources/StandardMacros.DoOnce` false :!label _label_2
    (:`Completed`
      (`|ExecutionSequence`
        (:`then_0`
          (`WidgetBlueprintLibrary.SetInputMode_GameAndUIEx` (`GameplayStatics.GetPlayerController` 0) null "DoNotLock" true true)
          (`/Engine/EditorBlueprintResources/StandardMacros.FlipFlop`
            (:`A`
              (`GameplayStatics.PlaySound2D` "/Game/Switch/SwitchBoard/SW_Panel_Switch_On.SW_Panel_Switch_On" 1.0 1.0 0.0 null null)
              (set `self.Switch01On` true)
              (bind (_direction _value) (`Timeline|Switch Animation` :!label _label_3)
                (:`Update`
                  (`SceneComponent.K2_SetRelativeRotation` (`self.SM_Switch`) (`KismetMathLibrary.MakeRotator` _value) false false))
                (:`Finished`
                  (`self.Switch 01`)
                  (`self.Done`))))
            (:`B`
              (`GameplayStatics.PlaySound2D` "/Game/Switch/SwitchBoard/SW_Panel_Switch_Off.SW_Panel_Switch_Off" 1.0 1.0 0.0 null null)
              (set `self.Switch01On` false)
              (goto _label_3 :!via `Reverse`))))
        (:`then_1`
          (`KismetSystemLibrary.Delay` 0.3)
          (goto _label_2 :!via `Reset`))))))

(event `Switch 01`
  (bind _sm_board_needle (`self.SM_Board_Needle`))
  (bind (_needle01_rotation_roll _needle01_rotation_pitch) (`KismetMathLibrary.BreakRotator` (`self.needle01 Rotation`)))
  (bind _sm_board_needle1 (`self.SM_Board_Needle1`))
  (bind (_needle02_rotation_roll _needle02_rotation_pitch) (`KismetMathLibrary.BreakRotator` (`self.needle02 Rotation`)))
  (bind _sm_board_needle1_2 (`self.SM_Board_Needle1`))
  (bind (_needle02_rotation_roll_2 _needle02_rotation_pitch_2) (`KismetMathLibrary.BreakRotator` (`self.needle02 Rotation`)))
  (bind (_needle01_rotation_roll_2 _needle01_rotation_pitch_2) (`KismetMathLibrary.BreakRotator` (`self.needle01 Rotation`)))
  (bind _sm_board_needle_2 (`self.SM_Board_Needle`))
  (bind _returnvalue (+ _needle01_rotation_pitch -20.0))
  (bind _returnvalue_2 (- _needle01_rotation_pitch_2 20.0))
  (bind _returnvalue_3 (- _needle02_rotation_pitch -10.0))
  (bind _returnvalue_4 (- _needle02_rotation_pitch_2 10.0))
  (if (`self.Switch01On`)
    (`|ExecutionSequence`
      (:`then_0`
        (`KismetSystemLibrary.MoveComponentTo` _sm_board_needle (`SceneComponent.RelativeLocation` _sm_board_needle) (`KismetMathLibrary.MakeRotator` 180.0 _returnvalue 180.0))
        (set `self.needle01 Rotation` (`KismetMathLibrary.MakeRotator` 180.0 _returnvalue 180.0)))
      (:`then_1`
        (`KismetSystemLibrary.MoveComponentTo` _sm_board_needle1 (`SceneComponent.RelativeLocation` _sm_board_needle1) (`KismetMathLibrary.MakeRotator` 180.0 _returnvalue_3 180.0))
        (set `self.needle01 Rotation` (`KismetMathLibrary.MakeRotator` 180.0 _returnvalue_3 180.0))))
    (else
      (`|ExecutionSequence`
        (:`then_0`
          (`KismetSystemLibrary.MoveComponentTo` _sm_board_needle_2 (`SceneComponent.RelativeLocation` _sm_board_needle_2) (`KismetMathLibrary.MakeRotator` 180.0 _returnvalue_2 180.0))
          (set `self.needle01 Rotation` (`KismetMathLibrary.MakeRotator` 180.0 _returnvalue_2 180.0)))
        (:`then_1`
          (`KismetSystemLibrary.MoveComponentTo` _sm_board_needle1_2 (`SceneComponent.RelativeLocation` _sm_board_needle1_2) (`KismetMathLibrary.MakeRotator` 180.0 _returnvalue_4 180.0))
          (set `self.needle01 Rotation` (`KismetMathLibrary.MakeRotator` 180.0 _returnvalue_4 180.0)))))))

(event `self.SM_Switch1.OnClicked`
  (params (TouchedComponent :type "PrimitiveComponent Object Reference") (ButtonPressed :type "Key Structure"))
  (`KismetSystemLibrary.PrintString` "1")
  (`WidgetBlueprintLibrary.SetFocusToGameViewport`)
  (`/Engine/EditorBlueprintResources/StandardMacros.DoOnce` false :!label _label_4
    (:`Completed`
      (`|ExecutionSequence`
        (:`then_0`
          (`WidgetBlueprintLibrary.SetInputMode_GameAndUIEx` (`GameplayStatics.GetPlayerController` 0) null "DoNotLock" true true)
          (`/Engine/EditorBlueprintResources/StandardMacros.FlipFlop`
            (:`A`
              (`GameplayStatics.PlaySound2D` "/Game/Switch/SwitchBoard/SW_Panel_Switch_On.SW_Panel_Switch_On" 1.0 1.0 0.0 null null)
              (set `self.Switch02On` true)
              (bind (_direction _value) (`Timeline|Timeline` :!label _label_5)
                (:`Update`
                  (`SceneComponent.K2_SetRelativeRotation` (`self.SM_Switch1`) (`KismetMathLibrary.MakeRotator` _value) false false))
                (:`Finished`
                  (`self.Switch 02`)
                  (`self.Done`))))
            (:`B`
              (`GameplayStatics.PlaySound2D` "/Game/Switch/SwitchBoard/SW_Panel_Switch_Off.SW_Panel_Switch_Off" 1.0 1.0 0.0 null null)
              (set `self.Switch02On` false)
              (goto _label_5 :!via `Reverse`))))
        (:`then_1`
          (`KismetSystemLibrary.Delay` 0.3)
          (goto _label_4 :!via `Reset`))))))

(event `self.SM_Switch2.OnClicked`
  (params (TouchedComponent :type "PrimitiveComponent Object Reference") (ButtonPressed :type "Key Structure"))
  (`KismetSystemLibrary.PrintString` "3")
  (`WidgetBlueprintLibrary.SetFocusToGameViewport`)
  (`/Engine/EditorBlueprintResources/StandardMacros.DoOnce` false :!label _label_6
    (:`Completed`
      (`|ExecutionSequence`
        (:`then_0`
          (`WidgetBlueprintLibrary.SetInputMode_GameAndUIEx` (`GameplayStatics.GetPlayerController` 0) null "DoNotLock" true true)
          (`/Engine/EditorBlueprintResources/StandardMacros.FlipFlop`
            (:`A`
              (`GameplayStatics.PlaySound2D` "/Game/Switch/SwitchBoard/SW_Panel_Switch_On.SW_Panel_Switch_On" 1.0 1.0 0.0 null null)
              (set `self.Switch03On` true)
              (bind (_direction _newtrack_0) (`Timeline|Timeline_0` :!label _label_7)
                (:`Update`
                  (`SceneComponent.K2_SetRelativeRotation` (`self.SM_Switch2`) (`KismetMathLibrary.MakeRotator` _newtrack_0) false false))
                (:`Finished`
                  (`self.Switch 03`)
                  (`self.Done`))))
            (:`B`
              (`GameplayStatics.PlaySound2D` "/Game/Switch/SwitchBoard/SW_Panel_Switch_Off.SW_Panel_Switch_Off" 1.0 1.0 0.0 null null)
              (set `self.Switch03On` false)
              (goto _label_7 :!via `Reverse`))))
        (:`then_1`
          (`KismetSystemLibrary.Delay` 0.3)
          (goto _label_6 :!via `Reset`))))))

(event `self.SM_Switch3.OnClicked`
  (params (TouchedComponent :type "PrimitiveComponent Object Reference") (ButtonPressed :type "Key Structure"))
  (`KismetSystemLibrary.PrintString` "4")
  (`WidgetBlueprintLibrary.SetFocusToGameViewport`)
  (`/Engine/EditorBlueprintResources/StandardMacros.DoOnce` false :!label _label_8
    (:`Completed`
      (`|ExecutionSequence`
        (:`then_0`
          (`WidgetBlueprintLibrary.SetInputMode_GameAndUIEx` (`GameplayStatics.GetPlayerController` 0) null "DoNotLock" true true)
          (`/Engine/EditorBlueprintResources/StandardMacros.FlipFlop`
            (:`A`
              (`GameplayStatics.PlaySound2D` "/Game/Switch/SwitchBoard/SW_Panel_Switch_On.SW_Panel_Switch_On" 1.0 1.0 0.0 null null)
              (set `self.Switch04On` true)
              (bind (_direction _newtrack_0) (`Timeline|Timeline_1` :!label _label_9)
                (:`Update`
                  (`SceneComponent.K2_SetRelativeRotation` (`self.SM_Switch3`) (`KismetMathLibrary.MakeRotator` _newtrack_0) false false))
                (:`Finished`
                  (`self.Switch 04`)
                  (`self.Done`))))
            (:`B`
              (`GameplayStatics.PlaySound2D` "/Game/Switch/SwitchBoard/SW_Panel_Switch_Off.SW_Panel_Switch_Off" 1.0 1.0 0.0 null null)
              (set `self.Switch04On` false)
              (goto _label_9 :!via `Reverse`))))
        (:`then_1`
          (`KismetSystemLibrary.Delay` 0.3)
          (goto _label_8 :!via `Reset`))))))

(event `Switch 02`
  (bind _sm_board_needle (`self.SM_Board_Needle`))
  (bind (_needle01_rotation_roll _needle01_rotation_pitch) (`KismetMathLibrary.BreakRotator` (`self.needle01 Rotation`)))
  (bind _sm_board_needle1 (`self.SM_Board_Needle1`))
  (bind (_needle02_rotation_roll _needle02_rotation_pitch) (`KismetMathLibrary.BreakRotator` (`self.needle02 Rotation`)))
  (bind _sm_board_needle1_2 (`self.SM_Board_Needle1`))
  (bind (_needle02_rotation_roll_2 _needle02_rotation_pitch_2) (`KismetMathLibrary.BreakRotator` (`self.needle02 Rotation`)))
  (bind (_needle01_rotation_roll_2 _needle01_rotation_pitch_2) (`KismetMathLibrary.BreakRotator` (`self.needle01 Rotation`)))
  (bind _sm_board_needle_2 (`self.SM_Board_Needle`))
  (bind _returnvalue (- _needle02_rotation_pitch_2 25.0))
  (bind _returnvalue_2 (- _needle01_rotation_pitch_2 25.0))
  (bind _returnvalue_3 (+ _needle01_rotation_pitch 25.0))
  (bind _returnvalue_4 (- _needle02_rotation_pitch -25.0))
  (if (`self.Switch02On`)
    (`|ExecutionSequence`
      (:`then_0`
        (`KismetSystemLibrary.MoveComponentTo` _sm_board_needle (`SceneComponent.RelativeLocation` _sm_board_needle) (`KismetMathLibrary.MakeRotator` 180.0 _returnvalue_3 180.0))
        (set `self.needle01 Rotation` (`KismetMathLibrary.MakeRotator` 180.0 _returnvalue_3 180.0)))
      (:`then_1`
        (`KismetSystemLibrary.MoveComponentTo` _sm_board_needle1 (`SceneComponent.RelativeLocation` _sm_board_needle1) (`KismetMathLibrary.MakeRotator` 180.0 _returnvalue_4 180.0))
        (set `self.needle01 Rotation` (`KismetMathLibrary.MakeRotator` 180.0 _returnvalue_4 180.0))))
    (else
      (`|ExecutionSequence`
        (:`then_0`
          (`KismetSystemLibrary.MoveComponentTo` _sm_board_needle_2 (`SceneComponent.RelativeLocation` _sm_board_needle_2) (`KismetMathLibrary.MakeRotator` 180.0 _returnvalue_2 180.0))
          (set `self.needle01 Rotation` (`KismetMathLibrary.MakeRotator` 180.0 _returnvalue_2 180.0)))
        (:`then_1`
          (`KismetSystemLibrary.MoveComponentTo` _sm_board_needle1_2 (`SceneComponent.RelativeLocation` _sm_board_needle1_2) (`KismetMathLibrary.MakeRotator` 180.0 _returnvalue 180.0))
          (set `self.needle01 Rotation` (`KismetMathLibrary.MakeRotator` 180.0 _returnvalue 180.0)))))))

(event `Switch 03`
  (bind _sm_board_needle (`self.SM_Board_Needle`))
  (bind (_needle01_rotation_roll _needle01_rotation_pitch) (`KismetMathLibrary.BreakRotator` (`self.needle01 Rotation`)))
  (bind _sm_board_needle1 (`self.SM_Board_Needle1`))
  (bind (_needle02_rotation_roll _needle02_rotation_pitch) (`KismetMathLibrary.BreakRotator` (`self.needle02 Rotation`)))
  (bind _sm_board_needle1_2 (`self.SM_Board_Needle1`))
  (bind (_needle02_rotation_roll_2 _needle02_rotation_pitch_2) (`KismetMathLibrary.BreakRotator` (`self.needle02 Rotation`)))
  (bind (_needle01_rotation_roll_2 _needle01_rotation_pitch_2) (`KismetMathLibrary.BreakRotator` (`self.needle01 Rotation`)))
  (bind _sm_board_needle_2 (`self.SM_Board_Needle`))
  (bind _returnvalue (- _needle02_rotation_pitch -5.0))
  (bind _returnvalue_2 (- _needle02_rotation_pitch_2 5.0))
  (bind _returnvalue_3 (- _needle01_rotation_pitch_2 10.0))
  (bind _returnvalue_4 (+ _needle01_rotation_pitch 10.0))
  (if (`self.Switch03On`)
    (`|ExecutionSequence`
      (:`then_0`
        (`KismetSystemLibrary.MoveComponentTo` _sm_board_needle (`SceneComponent.RelativeLocation` _sm_board_needle) (`KismetMathLibrary.MakeRotator` 180.0 _returnvalue_4 180.0))
        (set `self.needle01 Rotation` (`KismetMathLibrary.MakeRotator` 180.0 _returnvalue_4 180.0)))
      (:`then_1`
        (`KismetSystemLibrary.MoveComponentTo` _sm_board_needle1 (`SceneComponent.RelativeLocation` _sm_board_needle1) (`KismetMathLibrary.MakeRotator` 180.0 _returnvalue 180.0))
        (set `self.needle01 Rotation` (`KismetMathLibrary.MakeRotator` 180.0 _returnvalue 180.0))))
    (else
      (`|ExecutionSequence`
        (:`then_0`
          (`KismetSystemLibrary.MoveComponentTo` _sm_board_needle_2 (`SceneComponent.RelativeLocation` _sm_board_needle_2) (`KismetMathLibrary.MakeRotator` 180.0 _returnvalue_3 180.0))
          (set `self.needle01 Rotation` (`KismetMathLibrary.MakeRotator` 180.0 _returnvalue_3 180.0)))
        (:`then_1`
          (`KismetSystemLibrary.MoveComponentTo` _sm_board_needle1_2 (`SceneComponent.RelativeLocation` _sm_board_needle1_2) (`KismetMathLibrary.MakeRotator` 180.0 _returnvalue_2 180.0))
          (set `self.needle01 Rotation` (`KismetMathLibrary.MakeRotator` 180.0 _returnvalue_2 180.0)))))))

(event `Switch 04`
  (bind _sm_board_needle (`self.SM_Board_Needle`))
  (bind (_needle01_rotation_roll _needle01_rotation_pitch) (`KismetMathLibrary.BreakRotator` (`self.needle01 Rotation`)))
  (bind _sm_board_needle1 (`self.SM_Board_Needle1`))
  (bind (_needle02_rotation_roll _needle02_rotation_pitch) (`KismetMathLibrary.BreakRotator` (`self.needle02 Rotation`)))
  (bind _sm_board_needle1_2 (`self.SM_Board_Needle1`))
  (bind (_needle02_rotation_roll_2 _needle02_rotation_pitch_2) (`KismetMathLibrary.BreakRotator` (`self.needle02 Rotation`)))
  (bind (_needle01_rotation_roll_2 _needle01_rotation_pitch_2) (`KismetMathLibrary.BreakRotator` (`self.needle01 Rotation`)))
  (bind _sm_board_needle_2 (`self.SM_Board_Needle`))
  (bind _returnvalue (- _needle02_rotation_pitch 13.0))
  (bind _returnvalue_2 (- _needle01_rotation_pitch 0.0))
  (bind _returnvalue_3 (- _needle02_rotation_pitch_2 -13.0))
  (if (`self.Switch04On`)
    (`|ExecutionSequence`
      (:`then_0`
        (`KismetSystemLibrary.MoveComponentTo` _sm_board_needle_2 (`SceneComponent.RelativeLocation` _sm_board_needle_2) (`KismetMathLibrary.MakeRotator` 180.0 (+ _needle01_rotation_pitch_2 0.0) 180.0))
        (set `self.needle01 Rotation` (`KismetMathLibrary.MakeRotator` 180.0 0.0 180.0)))
      (:`then_1`
        (`KismetSystemLibrary.MoveComponentTo` _sm_board_needle1_2 (`SceneComponent.RelativeLocation` _sm_board_needle1_2) (`KismetMathLibrary.MakeRotator` 180.0 _returnvalue_3 180.0))
        (set `self.needle01 Rotation` (`KismetMathLibrary.MakeRotator` 180.0 _returnvalue_3 180.0))))
    (else
      (`|ExecutionSequence`
        (:`then_0`
          (`KismetSystemLibrary.MoveComponentTo` _sm_board_needle (`SceneComponent.RelativeLocation` _sm_board_needle) (`KismetMathLibrary.MakeRotator` 180.0 _returnvalue_2 180.0))
          (set `self.needle01 Rotation` (`KismetMathLibrary.MakeRotator` 180.0 _returnvalue_2 180.0)))
        (:`then_1`
          (`KismetSystemLibrary.MoveComponentTo` _sm_board_needle1 (`SceneComponent.RelativeLocation` _sm_board_needle1) (`KismetMathLibrary.MakeRotator` 180.0 _returnvalue 180.0))
          (set `self.needle01 Rotation` (`KismetMathLibrary.MakeRotator` 180.0 _returnvalue 180.0)))))))

(fn `UserConstructionScript`)