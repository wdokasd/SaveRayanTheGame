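; Example quest target character that dies when another pawn overlaps its Box, reporting a "Kill" objective.
; The overlap passes that pawn to the ManagerQuestTarget component's TryFinishObjective, and an IsAlive flag limits this to one death.
; Death disables capsule collision and movement, then ragdolls the mesh from the pelvis down while ignoring the Camera channel.
; The construction script copies TargetName into the quest target component.
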(event `self.Box.OnComponentBeginOverlap`
  (params (OverlappedComponent :type "PrimitiveComponent Object Reference") (OtherActor :type "Actor Object Reference") (OtherComp :type "PrimitiveComponent Object Reference") (OtherBodyIndex :type Integer) (bFromSweep :type Boolean) (SweepResult :type "HitResult Structure (by ref)"))
  (if (!= self OtherActor)
    (if (`self.IsAlive`)
      (cast `Pawn` OtherActor)
      (`/Game/QuestManager/Blueprints/Components/Manager_QuestTarget.Try_Finish_Objective` (`self.Manager_QuestTarget`) "Kill" OtherActor)
      (`PrimitiveComponent.SetCollisionProfileName` (`self.Mesh`) "Ragdoll" true)
      (`PrimitiveComponent.SetCollisionResponseToChannel` (`self.Mesh`) "ECC_Camera" "ECR_Ignore")
      (`CharacterMovementComponent.SetMovementMode` (`self.CharacterMovement`) "MOVE_None" 0)
      (`PrimitiveComponent.SetCollisionEnabled` (`self.CapsuleComponent`) "NoCollision")
      (`SkeletalMeshComponent.SetAllBodiesBelowSimulatePhysics` (`self.Mesh`) "Pelvis" true true)
      (set `self.IsAlive` false))))

(fn `UserConstructionScript`
  (set `/Game/QuestManager/Blueprints/Components/Manager_QuestTarget.TargetName` (`self.TargetName`) (`self.Manager_QuestTarget`)))