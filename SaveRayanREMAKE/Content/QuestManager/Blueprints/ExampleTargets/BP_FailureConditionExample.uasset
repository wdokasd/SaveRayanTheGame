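; Example quest target actor that triggers a named quest failure condition when a pawn enters its box.
; On overlap, it gets the Quest Manager from the pawn's controller and calls TryTriggerFailureCondition with its ConditionName.
; The construction script shows the condition name on a text render component.
; An author comment notes that the same call works from any event, not only an overlap.
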(event `self.Box.OnComponentBeginOverlap`
  (params (OverlappedComponent :type "PrimitiveComponent Object Reference") (OtherActor :type "Actor Object Reference") (OtherComp :type "PrimitiveComponent Object Reference") (OtherBodyIndex :type Integer) (bFromSweep :type Boolean) (SweepResult :type "HitResult Structure (by ref)"))
  ;[1 1 1] Call This Function From Quest Manager Anywhere You Like. Doesn't Have To Be An Overlap Event
  (bind _aspawn (cast `Pawn` OtherActor))
  (bind _returnvalue (`Pawn.GetController` _aspawn))
  (`/Engine/EditorBlueprintResources/StandardMacros.IsValid` _returnvalue
    (:`Is Valid`
      (bind _returnvalue_2 (`/Game/QuestManager/Blueprints/Data/Libraries/ML_MissionComponent.Get_Quest_Manager` _returnvalue)
        (:`then`
          (`/Game/QuestManager/Blueprints/Components/Manager_Mission.Try_Trigger_Failure_Condition` _returnvalue_2 (`self.ConditionName`)))))))

(fn `UserConstructionScript`
  (`TextRenderComponent.K2_SetText` (`self.TextRender`) (`KismetTextLibrary.Conv_NameToText` (`self.ConditionName`))))