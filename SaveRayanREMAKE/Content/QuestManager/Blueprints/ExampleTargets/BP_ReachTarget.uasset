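; BP_ReachTarget is an example quest target that completes a "Reach" objective when an actor enters its trigger box.
; The box overlap passes the overlapping actor as the player pawn to the ManagerQuestTarget component's TryFinishObjective.
; The construction script sizes the box from BoxExtent, raises it by its half-height, and copies TargetName onto the component.
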(event `self.Box.OnComponentBeginOverlap`
  (params (OverlappedComponent :type "PrimitiveComponent Object Reference") (OtherActor :type "Actor Object Reference") (OtherComp :type "PrimitiveComponent Object Reference") (OtherBodyIndex :type Integer) (bFromSweep :type Boolean) (SweepResult :type "HitResult Structure (by ref)"))
  (`/Game/QuestManager/Blueprints/Components/Manager_QuestTarget.Try_Finish_Objective` (`self.Manager_QuestTarget`) "Reach" OtherActor))

(fn `UserConstructionScript`
  (bind (_boxextent_x _boxextent_y _boxextent_z) (`KismetMathLibrary.BreakVector` (`self.BoxExtent`)))
  (`BoxComponent.SetBoxExtent` (`self.Box`) (`self.BoxExtent`) true)
  (`SceneComponent.K2_AddRelativeLocation` (`self.Box`) (`KismetMathLibrary.MakeVector` 0.0 0.0 _boxextent_z) false false)
  (set `/Game/QuestManager/Blueprints/Components/Manager_QuestTarget.TargetName` (`self.TargetName`) (`self.Manager_QuestTarget`)))