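; Quest target component that registers its owning actor's target with BP_QuestManager and optionally makes it interactable.
; On BeginPlay it builds tagged overlap boxes from InteractionZones and a hidden screen-space prompt widget, and binds deregistration to owner EndPlay.
; Pawn overlaps set the prompt's text and position for that zone and notify the controller's quest manager.
; Helpers forward objective completion, toggle prompt visibility and switch zone collision by tag.
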(fn `Construct_Interaction_Widget`
  (`self.InteractionWidget`
    (:`then`
      _)
    (:`else`
      (bind _returnvalue (`|CreateWidget` "/Game/QuestManager/UserInterface/SingleElems/WB_Interaction_Widget.WB_Interaction_Widget_C"))
      (set `self.InteractionWidget` _returnvalue)))
  (`self.InteractionWidgetComponent`
    (:`then`
      _)
    (:`else`
      (bind _returnvalue_2 (`|AddComponentByClass` :`self` (`self.GetOwner`) :`Class` "/Script/UMG.WidgetComponent"))
      (set `self.InteractionWidgetComponent` _returnvalue_2)))
  (`WidgetComponent.SetWidget` (`self.InteractionWidgetComponent`) (`self.InteractionWidget`))
  (`WidgetComponent.SetWidgetSpace` (`self.InteractionWidgetComponent`) "Screen")
  (`WidgetComponent.SetDrawAtDesiredSize` (`self.InteractionWidgetComponent`) true)
  (`SceneComponent.SetVisibility` (`self.InteractionWidgetComponent`) false false))

(fn `Construct_InteractionBox`
  (locals (LocInteractionBox :type "BoxComponent Object Reference") (LocInteraction :type "/Game/QuestManager/Blueprints/Data/Structs/Struct_TargetInteraction Structure"))
  (bind _interactionboxes (`self.InteractionBoxes`))
  (bind ((`InteractionBoxExtent_5_60B6CD15407A6E0FC97C42AED18C9C1D` _interactionboxextent) (`InteractionBoxOffset_7_54B6274A44050BB3E92C11BAA722817B` _interactionboxoffset)) (break `/Game/QuestManager/Blueprints/Data/Structs/Struct_TargetInteraction` (`local.LocInteraction`)))
  (clear `PrimitiveComponent.OnComponentBeginOverlap` _interactionboxes)
  (clear `PrimitiveComponent.OnComponentEndOverlap` _interactionboxes)
  (`KismetArrayLibrary.Array_Clear` (`self.InteractionBoxes`))
  (for _array_element (`self.InteractionZones`)
    (set `local.LocInteraction` _array_element)
    (bind _returnvalue (`|AddComponentByClass` :`self` (`self.GetOwner`) :`Class` "/Script/Engine.BoxComponent"))
    (set `local.LocInteractionBox` _returnvalue)
    (`KismetArrayLibrary.Array_Add` (`self.InteractionBoxes`) (`local.LocInteractionBox`))
    (`KismetArrayLibrary.Array_Add` (`ActorComponent.ComponentTags` (`local.LocInteractionBox`)) (`.InteractionBoxTag_13_A0E11C7B407469EEE69C26B15642DEED` (break `/Game/QuestManager/Blueprints/Data/Structs/Struct_TargetInteraction` (`local.LocInteraction`))))
    (`SceneComponent.K2_AttachToComponent` (`local.LocInteractionBox`) (`Actor.RootComponent` (`self.GetOwner`)) "None" "SnapToTarget" "SnapToTarget" "SnapToTarget" true)
    (`|ExecutionSequence`
      (:`then_0`
        ;[1 1 1] Set Interaction Box Extent And Offset
        (`BoxComponent.SetBoxExtent` (`local.LocInteractionBox`) _interactionboxextent true)
        (`SceneComponent.K2_AddLocalOffset` (`local.LocInteractionBox`) (`KismetMathLibrary.MakeVector` (.x _interactionboxoffset) (.y _interactionboxoffset) (+ (.z _interactionboxoffset) (.z _interactionboxextent))) false false))
      (:`then_1`
        ;[1 1 1] Bind Overlap Events
        (add `PrimitiveComponent.OnComponentBeginOverlap` (`local.LocInteractionBox`) (`|CreateDelegate` :!event `On_Interaction_Begin_Overlap`))
        (add `PrimitiveComponent.OnComponentEndOverlap` (`local.LocInteractionBox`) (`|CreateDelegate` :!event `On_Interaction_End_Overlap`)))
      (:`then_2`
        (`SceneComponent.SetHiddenInGame` (`local.LocInteractionBox`) true false)))))

(fn `Get_InteractionZone_By_Tag`
  (params (Tag :type Name))
  (returns (ReturnValue :type "/Game/QuestManager/Blueprints/Data/Structs/Struct_TargetInteraction Structure"))
  (locals (LocReturn :type "/Game/QuestManager/Blueprints/Data/Structs/Struct_TargetInteraction Structure"))
  (for _array_element (`self.InteractionZones`)
    (if (== (`.InteractionBoxTag_13_A0E11C7B407469EEE69C26B15642DEED` (break `/Game/QuestManager/Blueprints/Data/Structs/Struct_TargetInteraction` _array_element)) (`local.Tag`))
      (set `local.LocReturn` _array_element)
      (break)))
  (return (`local.LocReturn`)))

(fn `On_Interaction_Begin_Overlap`
  (params (OverlappedComponent :type "PrimitiveComponent Object Reference") (OtherActor :type "Actor Object Reference") (OtherComp :type "PrimitiveComponent Object Reference") (OtherBodyIndex :type Integer) (bFromSweep :type Boolean) (SweepResult :type "HitResult Structure (by ref)"))
  (locals (LocManager :type "/Game/QuestManager/Blueprints/Components/Manager_Mission Object Reference"))
  (bind _aspawn (cast `Pawn` (`local.OtherActor`)))
  (bind _returnvalue (`Pawn.GetController` _aspawn))
  (`/Engine/EditorBlueprintResources/StandardMacros.IsValid` _returnvalue
    (:`Is Valid`
      (bind _returnvalue_2 (`/Game/QuestManager/Blueprints/Data/Libraries/ML_MissionComponent.Get_Quest_Manager` _returnvalue)
        (:`then`
          (set `local.LocManager` _returnvalue_2)
          (`|ExecutionSequence`
            (:`then_0`
              (bind _asbox_collision (cast `BoxComponent` (`local.OverlappedComponent`)))
              (bind _interactionwidgetcomponent (`self.InteractionWidgetComponent`)
                (:`then`
                  (bind _aswb_interaction_widget (cast `/Game/QuestManager/UserInterface/SingleElems/WB_Interaction_Widget` (`WidgetComponent.GetWidget` _interactionwidgetcomponent)))
                  (bind _output (`|GetArrayItem` (`self.InteractionBoxes`) (`KismetArrayLibrary.Array_Find` (`self.InteractionBoxes`) _asbox_collision)))
                  (bind ((`InteractionText_2_AF00C3DD405559EB30D12BA16D2E6022` _interactiontext) (`InteractionWidgetOffset_10_ED8DD1DD421E0032EEA232A0A01D742B` _interactionwidgetoffset)) (break `/Game/QuestManager/Blueprints/Data/Structs/Struct_TargetInteraction` (`self.Get_InteractionZone_By_Tag` (`|GetArrayItem` (`ActorComponent.ComponentTags` _output)))))
                  (`/Game/QuestManager/UserInterface/SingleElems/WB_Interaction_Widget.Set_Interaction_Text` _aswb_interaction_widget _interactiontext)
                  (`SceneComponent.K2_SetRelativeLocation` (`self.InteractionWidgetComponent`) (`SceneComponent.RelativeLocation` _output) false false)
                  (`SceneComponent.K2_AddLocalOffset` (`self.InteractionWidgetComponent`) _interactionwidgetoffset false false))
                (:`else`)))
            (:`then_1`
              (`/Game/QuestManager/Blueprints/Components/Manager_Mission.On_Interaction_Target_Begin_Overlap` (`local.LocManager`) self))))))))

(fn `On_Interaction_End_Overlap`
  (params (OverlappedComponent :type "PrimitiveComponent Object Reference") (OtherActor :type "Actor Object Reference") (OtherComp :type "PrimitiveComponent Object Reference") (OtherBodyIndex :type Integer))
  (locals (LocManager :type "/Game/QuestManager/Blueprints/Components/Manager_Mission Object Reference"))
  (bind _aspawn (cast `Pawn` (`local.OtherActor`)))
  (bind _returnvalue (`Pawn.GetController` _aspawn))
  (`/Engine/EditorBlueprintResources/StandardMacros.IsValid` _returnvalue
    (:`Is Valid`
      (bind _returnvalue_2 (`/Game/QuestManager/Blueprints/Data/Libraries/ML_MissionComponent.Get_Quest_Manager` _returnvalue)
        (:`then`
          (bind _output_get (set `local.LocManager` _returnvalue_2))
          (`/Game/QuestManager/Blueprints/Components/Manager_Mission.On_Interaction_Target_End_Overlap` _output_get self))))))

(fn `On_Quest_Target_Destroyed`
  (params (Actor :type "Actor Object Reference") (EndPlayReason :type "EEndPlayReason Enum" :default "Destroyed"))
  (`/Game/QuestManager/Blueprints/BP_QuestManager.Remove_Target` (`self.QuestManager`) self))

(fn `ReceiveBeginPlay`
  (`|ExecutionSequence`
    (:`then_0`
      (if (`self.IsInteractable`)
        (`self.Construct_InteractionBox`)
        (`self.Construct_Interaction_Widget`)))
    (:`then_1`
      (bind _returnvalue (`GameplayStatics.GetActorOfClass` "/Game/QuestManager/Blueprints/BP_QuestManager.BP_QuestManager_C"))
      (bind _output_get (set `self.QuestManager` _returnvalue))
      (`/Game/QuestManager/Blueprints/BP_QuestManager.Assign_Target` _output_get self))
    (:`then_2`
      (add `Actor.OnEndPlay` (`self.GetOwner`) (`|CreateDelegate` :!event `On_Quest_Target_Destroyed`)))
    (:`then_3`
      (`self.On_Manager_Constructed`))))

(fn `ReceiveTick`
  (params (DeltaSeconds :type "Float (single-precision)")))

(fn `Set_Interaction_Enabled`
  (params (Tag :type Name) (Enabled :type Boolean))
  (locals (LocBox :type "BoxComponent Object Reference"))
  (for _array_element (`self.InteractionBoxes`)
    (if (`KismetArrayLibrary.Array_Contains` (`ActorComponent.ComponentTags` _array_element) (`local.Tag`))
      (set `local.LocBox` _array_element)
      (break)))
  (`PrimitiveComponent.SetCollisionEnabled` (`local.LocBox`) (select `bool` (`local.Enabled`) :`false` "NoCollision" :`true` "QueryOnly" :!type "ECollisionEnabled Enum")))

(fn `Toggle_InteractionWidget`
  (params (bNewVisibility :type Boolean))
  (`SceneComponent.SetVisibility` (`self.InteractionWidgetComponent`) (`local.bNewVisibility`) false))

(fn `Try_Finish_Objective`
  (params (ObjectiveTag :type Name) (PlayerPawn :type "Actor Object Reference"))
  (returns (Success :type Boolean))
  (bind _aspawn (cast `Pawn` (`local.PlayerPawn`)))
  (bind _returnvalue (`/Game/QuestManager/Blueprints/Data/Libraries/ML_MissionComponent.Get_Quest_Manager` (`Pawn.GetController` _aspawn))
    (:`then`
      (bind _success (`/Game/QuestManager/Blueprints/Components/Manager_Mission.Try_Finish_Objective` _returnvalue (`local.ObjectiveTag`) (`self.TargetName`)))
      (return _success))
    (:`Failed`
      (return false))))