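; BP_QuestStartPoint is a placeable actor that marks a named start point for the quest system.
; On BeginPlay it finds the BP_QuestManager in the level, caches it and registers itself as a start point, then removes itself on EndPlay.
; Its construction script writes StartPointName to a text render component, labelling the point with its name.
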(event `self.ReceiveBeginPlay`
  ;[1 1 1] Assign Start Point On Begin Play
  (bind _returnvalue (`GameplayStatics.GetActorOfClass` "/Game/QuestManager/Blueprints/BP_QuestManager.BP_QuestManager_C"))
  (set `self.QuestManager` _returnvalue)
  (`/Game/QuestManager/Blueprints/BP_QuestManager.Add_StartPoint` (`self.QuestManager`) self))

(event `self.ReceiveEndPlay`
  (params (EndPlayReason :type "EEndPlayReason Enum" :default "Destroyed"))
  ;[1 1 1] Remove Start Point On End Play
  (`/Game/QuestManager/Blueprints/BP_QuestManager.Remove_StartPoint` (`self.QuestManager`) self))

(fn `UserConstructionScript`
  (`TextRenderComponent.K2_SetText` (`self.TextRender`) (`KismetTextLibrary.Conv_NameToText` (`self.StartPointName`))))